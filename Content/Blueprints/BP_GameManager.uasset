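; Game manager actor that holds player health and creates the on-screen HUD.
; On BeginPlay it adds a WBP_HUD widget to the viewport, assigns it the first BP_GameManager found in the level, and refreshes the counter text.
; SetHealthSafe clamps health between zero and MaxHealth, then pushes a counter text update to the HUD.
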(event `self.ReceiveBeginPlay`
  (bind _returnvalue (`|CreateWidget` "/Game/LevelPrototyping/Meshes/WBP_HUD.WBP_HUD_C" (`GameplayStatics.GetPlayerController` 0)))
  (bind _outactors (`GameplayStatics.GetAllActorsOfClass` "BP_GameManager_C"))
  (`UserWidget.AddToViewport` _returnvalue 0)
  (set `/Game/LevelPrototyping/Meshes/WBP_HUD.GameManager` (`|GetArrayItem` _outactors) _returnvalue)
  (bind _output_get (set `self.HUDRef` _returnvalue))
  (`/Game/LevelPrototyping/Meshes/WBP_HUD.UpdateCounterText` _output_get))

(event `self.ReceiveTick`
  (params (DeltaSeconds :type "Float (single-precision)")))

(fn `SetHealthSafe`
  (params (NewValue :type Integer))
  (set `self.Health` (`KismetMathLibrary.Clamp` NewValue 0 (`self.MaxHealth`)))
  (`/Game/LevelPrototyping/Meshes/WBP_HUD.UpdateCounterText` (`self.HUDRef`)))

(fn `UserConstructionScript`)